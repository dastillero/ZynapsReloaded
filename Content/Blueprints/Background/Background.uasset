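; Scrolling background actor that stays behind the camera along the world Y axis and fakes movement by scrolling its texture.
; The construction script builds a dynamic instance of the scrolling background material, assigns the configured texture with zeroed offsets and applies it to the static mesh.
; Every tick it snaps to the camera's Y position and drives the material's OffsetX from that position scaled by a speed multiplier.
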(event EventTick
  (params (DeltaSeconds :type Float%20%28single-precision%29))
  (bind _returnvalue (Transformation|GetActorLocation))
  ;[1 1 1] Follow camera
  (Transformation|SetActorLocation (Math|Vector|MakeVector (.x _returnvalue) (.y (Camera|GetCameraLocation (Game|GetPlayerCameraManager 0))) (.z _returnvalue)) false false)
  ;[1 1 1] Scroll background texture
  (Rendering|Material|SetScalarParameterValue (Variables|Default|GetDynamicMaterial) "OffsetX" (* (.y (Camera|GetCameraLocation (Variables|/Script/Engine.PlayerController|GetPlayerCameraManager (Game|GetPlayerController 0)))) (Variables|Default|GetScrollSpeedMultiplier)) :!class /Script/Engine.MaterialInstanceDynamic))

(fn ConstructionScript
  ;[1 1 1] Configure and set the dynamic material instance
  (bind _returnvalue (Rendering|Material|CreateDynamicMaterialInstance "/Game/Materials/Backgrounds/Mat_ScrollingBG.Mat_ScrollingBG" :!class /Script/Engine.KismetMaterialLibrary))
  (Rendering|Material|SetTextureParameterValue _returnvalue "Texture" (Variables|Default|GetTexture))
  (Rendering|Material|SetScalarParameterValue _returnvalue "OffsetX" 0.0 :!class /Script/Engine.MaterialInstanceDynamic)
  (Rendering|Material|SetScalarParameterValue _returnvalue "OffsetY" 0.0 :!class /Script/Engine.MaterialInstanceDynamic)
  (Rendering|Material|SetMaterial (Variables|Debug|GetStaticMeshComponent) 0 _returnvalue)
  (Variables|Default|SetDynamicMaterial _returnvalue))