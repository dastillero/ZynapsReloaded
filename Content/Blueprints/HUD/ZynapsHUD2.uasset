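; HUD class for Zynaps that shows screen widgets matching the current game state.
; BeginPlay creates the PrepareForCombat, GameOver and HUDFrame widgets and puts the frame on screen immediately.
; Each DrawHUD pass reads the state from ZynapsGameState, adding the prepare screen while Preparing, removing it while Playing, and adding the game over screen on Game Over.
; Viewport checks guard these per-frame adds and removes against repeats.
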(event EventDrawHUD
  (params (SizeX :type Integer) (SizeY :type Integer))
  (bind _aszynaps_game_state (Utilities|Casting|CastToZynapsGameState (Game|GetGameState)))
  (switch Utilities|FlowControl|Switch|SwitchonEStageState (Class|ZynapsGameState|GetCurrentState _aszynaps_game_state)
    (:Preparing
      (CallFunction|DrawPreparing))
    (:Playing
      (CallFunction|DrawPlaying))
    (:GameOver
      (CallFunction|DrawGameOver))))

(event EventBeginPlay
  (bind _returnvalue (UserInterface|CreateWidget "/Game/Blueprints/HUD/PrepareForCombat.PrepareForCombat_C"))
  (Variables|Default|SetPrepareForCombat _returnvalue)
  (bind _returnvalue_2 (UserInterface|CreateWidget "/Game/Blueprints/HUD/GameOver.GameOver_C"))
  (Variables|Default|SetGameOver _returnvalue_2)
  (bind _returnvalue_3 (UserInterface|CreateWidget "/Game/Blueprints/HUD/HUDFrame.HUDFrame_C"))
  (bind _output_get (Variables|Default|SetHUDFrame _returnvalue_3))
  (UserInterface|Viewport|AddtoViewport _output_get 0))

(fn ConstructionScript)

(fn DrawPreparing
  (bind _prepareforcombat (Variables|Default|GetPrepareForCombat))
  (if (not (UserInterface|Viewport|IsinViewport _prepareforcombat))
    (UserInterface|Viewport|AddtoViewport _prepareforcombat 0)))

(fn DrawPlaying
  (bind _prepareforcombat (Variables|Default|GetPrepareForCombat))
  (if (UserInterface|Viewport|IsinViewport _prepareforcombat)
    (Widget|RemovefromParent _prepareforcombat)))

(fn DrawGameOver
  (bind _gameover (Variables|Default|GetGameOver))
  (if (not (UserInterface|Viewport|IsinViewport _gameover))
    (UserInterface|Viewport|AddtoViewport _gameover 0)))